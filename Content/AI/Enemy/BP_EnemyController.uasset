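; AI controller for enemies that runs BT_Enemy and chooses which player or ally character to chase.
; Perception updates maintain a Targets list and the IsSensingAPlayer blackboard key.
; SetBestTarget runs on those updates and a 0.1-second loop, writing Target using estimated catch-up time (distance over speed difference).
; An alternative closest-target mode exists, but its test compares distance against zero, so it never selects anyone.
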(event OnTargetPerceptionUpdated(AIPerception)
  (params (Actor :type Actor%20Object%20Reference) (Stimulus :type AI%20Stimulus%20Structure))
  (bind _returnvalue (AI|GetBlackboard 0))
  (bind _returnvalue_2 (Utilities|Name|MakeLiteralName "IsSensingAPlayer"))
  (bind _targets (Variables|Default|GetTargets))
  ;[1 1 1] Find targets
  (bind _ascharacter (Utilities|Casting|CastToCharacter Actor))
  (Utilities|Casting|CastToBP_PlayerCharacter Actor
    (:then
      _)
    (:CastFailed
      (Utilities|Casting|CastToBP_AllyCharacter Actor)))
  (if (.bSuccessfullySensed (Utilities|Struct|BreakAIStimulus Stimulus))
    (Utilities|Array|AddUnique _targets _ascharacter)
    (AI|Components|Blackboard|SetValueasBool _returnvalue _returnvalue_2 true)
    (CallFunction|SetBestTarget (Variables|Default|GetTargetChaseAlgorithm) :!label _label)
    (else
      (Utilities|Array|RemoveItem _targets _ascharacter)
      (if (== (Utilities|Array|Length _targets) 0)
        (AI|Components|Blackboard|SetValueasBool _returnvalue _returnvalue_2 false)
        (goto _label)))))

(event EventBeginPlay
  ;[1 1 1] Blackboard Initial setup for Enemy
  (Utilities|FlowControl|Sequence
    (:then_0
      (Variables|Default|SetTargetChaseAlgorithm "NewEnumerator1")
      (Class|AIController|UseBlackboard "/Game/AI/Enemy/BB_Enemy.BB_Enemy")
      (AI|RunBehaviorTree "/Game/AI/Enemy/BT_Enemy.BT_Enemy"))
    (:then_1
      ;;[1 1 1] Looping for Best target value change
      (Utilities|FlowControl|Delay 0.1 :!label _label)
      (CallFunction|SetBestTarget (Variables|Default|GetTargetChaseAlgorithm))
      (goto _label))))

(fn ConstructionScript)

(fn SetBestTarget
  (params (AlgorithmType :type TargetCatchTypes%20Enum))
  (bind _returnvalue (Utilities|Name|MakeLiteralName "Target"))
  (bind _self self)
  (bind _returnvalue_2 (AI|GetBlackboard _self))
  (bind _output_get (LocalVariables|SetAlgorithType AlgorithmType))
  (if (Utilities|Enum|Equal(Enum) _output_get "NewEnumerator0")
    (LocalVariables|SetBestTargetValue 3e+03) ; I have no idea how to check sight radius
    (else
      (LocalVariables|SetBestTargetValue 9999.0)))
  (bind _asbp_enemy_character (Utilities|Casting|CastToBP_EnemyCharacter (Pawn|GetControlledPawn)))
  (LocalVariables|SetSelfCharacter _asbp_enemy_character)
  (for _array_element (Variables|Default|GetTargets)
    (LocalVariables|SetCurrentArrayObject _array_element)
    (if (Utilities|Enum|Equal(Enum) (LocalVariables|GetAlgorithType) "NewEnumerator0")
      ;[1 1 1] Best Target calculation algorithms
      (bind (_isbetter _newvalue) (CallFunction|ClosestTarget (LocalVariables|GetSelfCharacter) (LocalVariables|GetCurrentArrayObject) (LocalVariables|GetBestTargetValue)))
      (if _isbetter
        (LocalVariables|SetBestTargetValue _newvalue)
        (LocalVariables|SetBestTargetObject (LocalVariables|GetCurrentArrayObject) :!label _label))
      (else
        (bind (_isbetter_2 _newvalue_2) (CallFunction|VelocityandDistanceRatio (LocalVariables|GetSelfCharacter) (LocalVariables|GetCurrentArrayObject) (LocalVariables|GetBestTargetValue)))
        (if _isbetter_2
          (LocalVariables|SetBestTargetValue _newvalue_2)
          (goto _label)))))
  ;[1 1 1] Set New Target
  (if (!= (AI|Components|Blackboard|GetValueasObject _returnvalue_2 _returnvalue) (LocalVariables|GetBestTargetObject))
    (AI|Components|Blackboard|SetValueasObject _returnvalue_2 _returnvalue (LocalVariables|GetBestTargetObject))))

(fn VelocityandDistanceRatio
  (params (Seeker :type Character%20Object%20Reference%20%28by%20ref%29) (Target :type Character%20Object%20Reference%20%28by%20ref%29) (CurrentBestValue :type Float%20%28single-precision%29))
  (bind _returnvalue (Transformation|GetVelocity Target))
  (bind _charactermovement (Variables|/Script/Engine.Character|GetCharacterMovement Seeker))
  (bind _returnvalue_2 (Math|Vector|VectorLength _returnvalue))
  (bind _maxwalkspeed (Variables|/Script/Engine.CharacterMovementComponent|GetMaxWalkSpeed _charactermovement))
  (bind _returnvalue_3 (- _maxwalkspeed _returnvalue_2))
  (if (> _returnvalue_3 0.0)
    (LocalVariables|SetTempValue (/ (Math|Vector|VectorLength (- (Transformation|GetWorldLocation (Variables|/Script/Engine.Character|GetCapsuleComponent Seeker)) (Transformation|GetWorldLocation (Variables|/Script/Engine.Character|GetCapsuleComponent Target)))) _returnvalue_3))
    (else
      (LocalVariables|SetTempValue 9998.0)))
  (return (> CurrentBestValue (LocalVariables|GetTempValue)) (LocalVariables|GetTempValue)))

(fn ClosestTarget
  (params (Seeker :type Character%20Object%20Reference%20%28by%20ref%29) (Target :type Character%20Object%20Reference%20%28by%20ref%29) (CurrentBestValue :type Float%20%28single-precision%29))
  (bind _capsulecomponent (Variables|/Script/Engine.Character|GetCapsuleComponent Target))
  (bind _capsulecomponent_2 (Variables|/Script/Engine.Character|GetCapsuleComponent Seeker))
  (bind _returnvalue (Transformation|GetWorldLocation _capsulecomponent))
  (bind _returnvalue_2 (Transformation|GetWorldLocation _capsulecomponent_2))
  (bind _returnvalue_3 (- _returnvalue_2 _returnvalue))
  (bind _returnvalue_4 (Math|Vector|VectorLength _returnvalue_3))
  (return (> 0.0 _returnvalue_4) _returnvalue_4))