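; Goblin enemy character that chases the player within a leash range of its spawn point, takes damage and drops loot on death.
; AttackPlayer loops AIMoveTo toward the player, heading back to the spawn position saved at construction when too far.
; Lethal AnyDamage triggers Die, which spawns a randomized BP_ItemPack and destroys the actor.
; Idle wandering, player detection and attack animation are disconnected, leaving DoAttack and PlayerLost empty.
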(event Custom|enemyIdleMovement
  ;[1 1 1] Disabled for AI tests
  ;;[1 1 1] Enemy idle movement
)

(event Custom|Die
  ;[1 1 1] Enemy dies
  (Development|PrintString (Utilities|String|BuildString(Name) "" "" (Variables|Attributes|GetName) "has been slane"))
  (bind _returnvalue (Game|SpawnActorfromClass "/Game/Items/BP_ItemPack.BP_ItemPack_C" (Transformation|GetWorldTransform (Variables|Character|GetMesh)) "Undefined" self 0))
  (Default|RandomizeData _returnvalue)
  (Default|SetTexttoItemTextWidget _returnvalue (.name (Variables|/Game/Items/BP_ItemPack.BP_ItemPack_C|GetData _returnvalue)))
  (Actor|DestroyActor))

(event Custom|attackPlayer
  ;[1 1 1] Disabled for AI tests
  ;;[1 1 1] Enemy attack player
  (Variables|Default|SetisIdle false)
  (Variables|Default|SetisDuringAttack true)
  (Variables|/Script/Engine.CharacterMovementComponent|SetMaxWalkSpeed (Variables|Character|GetCharacterMovement) 4e+02)
  (if (< (Math|Float|Absolute(Float) (Math|Vector|VectorLength (- (Variables|Default|GetspawnPosition) (Transformation|GetActorLocation)))) 1e+03) :!label _label
    ;;;[1 1 1] Enemy going to Players location
    (if (< (Math|Float|Absolute(Float) (Math|Vector|VectorLength (- (Transformation|GetActorLocation) (Transformation|GetActorLocation (Game|GetPlayerCharacter 0))))) 1e+02)
      (CallFunction|DoAttack)
      (else
        (AI|AIMoveTo self "0, 0, 0" (Game|GetPlayerCharacter 0) 1.0 false
          (:then
            (Utilities|FlowControl|Delay 0.2)
            (goto _label)))))
    (else
      ;;;[1 1 1] Enemy went too far away - back to spawn
      (Variables|Default|SetisDuringAttack false)
      (AI|AIMoveTo self (Variables|Default|GetspawnPosition) 0 5.0 false
        (:OnSuccess
          (CallFunction|PlayerLost))))))

(event Custom|doAttack
  ;[1 1 1] Disabled for AI tests
  ;;[1 1 1] Enemy attack player
)

(event Custom|playerLost
  ;[1 1 1] Disabled for AI tests
  ;;[1 1 1] Enemy idle movement
)

(event Game|Damage|EventAnyDamage
  (params (Damage :type Float%20%28single-precision%29) (DamageType :type Damage%20Type%20Object%20Reference) (InstigatedBy :type Controller%20Object%20Reference) (DamageCauser :type Actor%20Object%20Reference))
  ;[1 1 1] Apply damage
  (if (not (Variables|Default|GetisDead))
    (if (<= (- (Variables|Attributes|GetHealth) Damage) 0.0)
      (Variables|Default|SetisDead true)
      (CallFunction|Die)
      (else
        (bind _output_get (Variables|Attributes|SetHealth (- (Variables|Attributes|GetHealth) Damage)))
        (Development|PrintString (Utilities|String|ToString(Float) _output_get))))))

(event EventBeginPlay
  ;[1 1 1] Disabled for AI tests
)

(fn ConstructionScript
  (Variables|Default|SetspawnPosition (Transformation|GetActorLocation))
  (Variables|Default|SetisIdle true))