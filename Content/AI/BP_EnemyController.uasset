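; BP_EnemyController is the AI controller that drives enemies through the BT_Enemy behavior tree.
; On BeginPlay it sets up BB_Enemy, stores player character 0 as the Target, then runs the tree.
; AI Perception updates that involve a BP_PlayerCharacter write the sensed result to the IsSensingAPlayer blackboard key, while the Target key stays as first set.
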(event OnTargetPerceptionUpdated(AIPerception)
  (params (Actor :type Actor%20Object%20Reference) (Stimulus :type AI%20Stimulus%20Structure))
  ;[1 1 1] Find a player
  (Utilities|Casting|CastToBP_PlayerCharacter Actor)
  (AI|Components|Blackboard|SetValueasBool (AI|GetBlackboard 0) (Utilities|Name|MakeLiteralName "IsSensingAPlayer") (.bSuccessfullySensed (Utilities|Struct|BreakAIStimulus Stimulus))))

(event EventBeginPlay
  ;[1 1 1] Blackboard Initial setup for Enemy
  (bind _blackboardcomponent (Class|AIController|UseBlackboard "/Game/AI/BB_Enemy.BB_Enemy"))
  (AI|Components|Blackboard|SetValueasObject _blackboardcomponent (Utilities|Name|MakeLiteralName "Target") (Game|GetPlayerCharacter 0))
  (AI|RunBehaviorTree "/Game/AI/BT_Enemy.BT_Enemy"))

(fn ConstructionScript)